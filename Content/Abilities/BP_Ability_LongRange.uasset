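; BP_Ability_LongRange is a character ability that plays the AM_LongRange montage on its owner's mesh when activated.
; Initialize runs the parent setup, then binds handlers to the activated, deactivated and interrupted events.
; When the montage completes, the ability asks the owner's AbilityManagerComponent to deactivate it by its gameplay tag.
; The deactivate and interrupt handlers are empty, and only the montage's Completed output is handled.
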(event Custom|On%20Activate
  (params (AbilityGameplayTag :type Gameplay%20Tag%20Structure%20%28by%20ref%29) (AbilityPtr :type Character%20Ability%20Base%20Object%20Reference))
  (Animation|Montage|PlayMontage (Variables|/Script/Engine.Character|GetMesh (Variables|Default|GetOwnerCharacter)) "/Game/Abilities/Montages/AM_LongRange.AM_LongRange"
    (:OnCompleted
      (bind _returnvalue (Class|CharacterAbilityBase|GetAbilityGameplayTag))
      (Class|AbilityManagerComponent|TryDeactivateAvilitywithTag (Variables|/Script/RPG.CharacterBase|GetAbilityManagerComponent (Variables|Default|GetOwnerCharacter)) _returnvalue))))

(event Custom|On%20Deactivate
  (params (AbilityGameplayTag :type Gameplay%20Tag%20Structure%20%28by%20ref%29) (AbilityPtr :type Character%20Ability%20Base%20Object%20Reference)))

(event Custom|On%20Interrupted
  (params (AbilityGameplayTag :type Gameplay%20Tag%20Structure%20%28by%20ref%29) (AbilityPtr :type Character%20Ability%20Base%20Object%20Reference)))

(event EventInitialize
  (params (InOwnerCharacter :type Character%20Base%20Object%20Reference))
  (|CallParentFunction InOwnerCharacter)
  (EventDispatchers|BindEventtoOnAbilityActivated (delegate Custom|On%20Activate))
  (EventDispatchers|BindEventtoOnAbilityDeactivated (delegate Custom|On%20Deactivate))
  (EventDispatchers|BindEventtoOnAbilityInterrputed (delegate Custom|On%20Interrupted)))