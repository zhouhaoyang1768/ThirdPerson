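; Plate projectile ability actor that damages characters it overlaps.
; On BeginPlay it launches horizontally along its owner's forward vector by setting the ProjectileMovement velocity.
; Overlapping any CharacterBase other than the owner calls HandleDamage with fixed damage and interrupt intensity, without destroying the projectile.
; Tick counts down LifeTime and destroys the actor when it runs out.
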(event EventBeginPlay
  (Variables|/Script/Engine.MovementComponent|SetVelocity (Variables|Default|GetProjectileMovement) (* (Transformation|GetActorForwardVector (Components|GetOwner)) "1500.000000,1500.000000,0.000000")))

(event Collision|EventActorBeginOverlap
  (params (OtherActor :type Actor%20Object%20Reference))
  (if (!= OtherActor (Components|GetOwner))
    (bind _ascharacter_base (Utilities|Casting|CastToCharacterBase OtherActor))
    (Class|CharacterBase|HandleDamage _ascharacter_base 0 1e+02 0.33)))

(event EventTick
  (params (DeltaSeconds :type Float%20%28single-precision%29))
  (bind _output_get (Variables|Default|SetLifeTime (- (Variables|Default|GetLifeTime) DeltaSeconds)))
  (if (<= _output_get 0.0)
    (Actor|DestroyActor)))

(fn ConstructionScript)