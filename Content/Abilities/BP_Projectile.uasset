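; BP_Projectile is an ability projectile that explodes on overlap and destroys itself when its lifetime runs out.
; Tick manually integrates acceleration into velocity and position without sweep, and combines accumulated spin with a velocity-based look-at rotation.
; While Expanding is set, it grows uniformly and ignores overlaps.
; Otherwise, overlapping any actor except its owner spawns BP_Explosion at its transform and destroys it.
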(event EventBeginPlay)

(event EventTick
  (params (DeltaSeconds :type Float%20%28single-precision%29))
  (CallFunction|UpdateTranslation DeltaSeconds)
  (CallFunction|UpdateRotation DeltaSeconds)
  (CallFunction|UpdateScale DeltaSeconds)
  (bind _output_get (Variables|Default|SetLifeTime (- (Variables|Default|GetLifeTime) DeltaSeconds)))
  (if (<= _output_get 0.0)
    (Actor|DestroyActor)))

(event Collision|EventActorBeginOverlap
  (params (OtherActor :type Actor%20Object%20Reference))
  (Development|PrintString "begin overlap")
  (if (and (!= OtherActor (Components|GetOwner)) (not (Variables|Default|GetExpanding)))
    (Development|PrintString "overlap")
    (Game|SpawnActorfromClass "/Game/Combat/Attack/BP_Explosion.BP_Explosion_C" (Transformation|GetActorTransform) "Undefined" "MultiplyWithRoot" 0 0)
    (Actor|DestroyActor)))

(fn ConstructionScript)

(fn UpdateTranslation
  (params (dt :type Float%20%28double-precision%29))
  (bind _output_get (Variables|Default|SetVelocity (+ (* (Variables|Default|GetAcceleration) dt) (Variables|Default|GetVelocity))))
  (Transformation|SetActorLocation (+ (* _output_get dt) (Transformation|GetActorLocation)) false false))

(fn UpdateRotation
  (params (dt :type Float%20%28double-precision%29))
  (bind _output_get (Variables|Default|SetRotation (Math|Rotator|CombineRotators (Variables|Default|GetRotation) (* (Variables|Default|GetAngularVelocity) dt))))
  (Transformation|SetActorRotation (Math|Rotator|CombineRotators _output_get (Math|Rotator|FindLookatRotation (Class|KismetMathLibrary|VectorForward) (Variables|Default|GetVelocity)))))

(fn UpdateScale
  (params (dt :type Float%20%28double-precision%29))
  (if (Variables|Default|GetExpanding)
    (Transformation|SetActorScale3D (+ (Transformation|GetActorScale3D) (Math|Vector|MakeVector dt dt dt)))))