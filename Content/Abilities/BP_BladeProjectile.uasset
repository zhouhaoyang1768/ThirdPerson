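; Blade projectile ability actor that damages characters it overlaps, other than its owner.
; On BeginPlay it sets its movement velocity from the owner's forward vector, negated and flattened to horizontal.
; Overlapping a CharacterBase applies damage through its HealthComponent and raises HitReactComponent intensity, without destroying the projectile.
; Tick counts down LifeTime and destroys the actor when it expires.
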(event EventBeginPlay
  (Variables|/Script/Engine.MovementComponent|SetVelocity (Variables|Default|GetProjectileMovement) (* (Transformation|GetActorForwardVector (Components|GetOwner)) "-100.000000,-100.000000,0.000000")))

(event Collision|EventActorBeginOverlap
  (params (OtherActor :type Actor%20Object%20Reference))
  (if (!= OtherActor (Components|GetOwner))
    (bind _ascharacter_base (Utilities|Casting|CastToCharacterBase OtherActor))
    (Class|HealthComponent|TakeDamage (Variables|/Script/RPG.CharacterBase|GetHealthComponent _ascharacter_base) 1e+02)
    (Class|HitReactComponent|IncreaseIntensity (Variables|/Script/RPG.CharacterBase|GetHitReactComponent _ascharacter_base) 0.33)))

(event EventTick
  (params (DeltaSeconds :type Float%20%28single-precision%29))
  (bind _output_get (Variables|Default|SetLife%20Time (- (Variables|Default|GetLife%20Time) DeltaSeconds)))
  (if (<= _output_get 0.0)
    (Actor|DestroyActor)))

(fn ConstructionScript)