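; Fireball ability that grows a projectile while active and launches it when deactivated.
; Binds the ability's activate, deactivate and interrupt events on initialize.
; Activation plays the charge montage and has the BP_ThirdPersonCharacter owner spawn a spinning, expanding fireball; the ability's own SpawnFireball is empty.
; Deactivation launches it along the owner's forward vector with an attack montage, while interruption destroys it.
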(event Custom|On%20Activate
  (params (AvilityGameplayTag :type Gameplay%20Tag%20Structure%20%28by%20ref%29) (AbilityPtr :type Character%20Ability%20Base%20Object%20Reference))
  (Animation|Montage|PlayMontage (Variables|/Script/Engine.Character|GetMesh (Variables|Default|GetOwnerCharacter)) "/Game/Variant_Combat/Anims/AM_ChargedAttack.AM_ChargedAttack"
    (:then
      (bind _asbp_third_person_character (Utilities|Casting|CastToBP_ThirdPersonCharacter (Variables|Default|GetOwnerCharacter)))
      (bind _projectile (Default|SpawnFireball _asbp_third_person_character))
      (bind _output_get (Variables|Default|SetFireball _projectile))
      (Variables|/Game/Abilities/BP_Projectile.BP_Projectile_C|SetAngularVelocity _output_get "0.000000,360.000000,0.000000")
      (Variables|Default|SetActive true)
      (Variables|/Game/Abilities/BP_Projectile.BP_Projectile_C|SetExpanding _projectile true))))

(event Custom|On%20Deactivate
  (params (AvilityGameplayTag :type Gameplay%20Tag%20Structure%20%28by%20ref%29) (AbilityPtr :type Character%20Ability%20Base%20Object%20Reference))
  (if (Variables|Default|GetActive)
    (Animation|StopAnimMontage (Variables|Default|GetOwnerCharacter) "/Game/Variant_Combat/Anims/AM_ChargedAttack.AM_ChargedAttack")
    (Variables|/Game/Abilities/BP_Projectile.BP_Projectile_C|SetVelocity (Variables|Default|GetFireball) (* (Math|Vector|GetForwardVector (Transformation|GetActorRotation (Variables|Default|GetOwnerCharacter))) "500.000000,500.000000,500.000000"))
    (Variables|/Game/Abilities/BP_Projectile.BP_Projectile_C|SetExpanding (Variables|Default|GetFireball) false)
    (Variables|Default|SetFireball 0)
    (Variables|Default|SetActive false)
    (Animation|PlayAnimMontage (Variables|Default|GetOwnerCharacter) "/Game/Arena/Anims/AM_NormalAttack1.AM_NormalAttack1" 1.0 "None")))

(event Custom|On%20Interrupted
  (params (AvilityGameplayTag :type Gameplay%20Tag%20Structure%20%28by%20ref%29) (AbilityPtr :type Character%20Ability%20Base%20Object%20Reference))
  (Animation|StopAnimMontage (Variables|Default|GetOwnerCharacter) "/Game/Variant_Combat/Anims/AM_ChargedAttack.AM_ChargedAttack")
  (Actor|DestroyActor (Variables|Default|GetFireball))
  (Variables|Default|SetActive false))

(event EventInitialize
  (params (InOwnerCharacter :type Character%20Base%20Object%20Reference))
  (|CallParentFunction InOwnerCharacter)
  (EventDispatchers|BindEventtoOnAbilityActivated (delegate Custom|On%20Activate))
  (EventDispatchers|BindEventtoOnAbilityDeactivated (delegate Custom|On%20Deactivate))
  (EventDispatchers|BindEventtoOnAbilityInterrputed (delegate Custom|On%20Interrupted)))

(fn SpawnFireball)