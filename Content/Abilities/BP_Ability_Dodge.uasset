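; Dodge ability that grants the owning character brief damage immunity and plays a directional dodge montage on activation.
; GetDirection measures the signed angle from actor forward to last movement input as 0–360 degrees, defaulting to forward without input.
; GetSector splits the circle into equal, centered sectors sized by the Animations array length to select the montage.
; Montage completion or interruption asks the AbilityManagerComponent to deactivate the ability by tag.
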(event Custom|On%20Activate
  (params (AbilityGameplayTag :type Gameplay%20Tag%20Structure%20%28by%20ref%29) (AbilityPtr :type Character%20Ability%20Base%20Object%20Reference))
  (bind _ownercharacter (Variables|Default|GetOwnerCharacter))
  (Class|HealthComponent|SetImmuneTime (Variables|/Script/RPG.CharacterBase|GetHealthComponent (Variables|Default|GetOwnerCharacter)) 1.5)
  (bind _angle (CallFunction|GetDirection))
  (bind _sector (CallFunction|GetSector _angle))
  (Animation|Montage|PlayMontage (Variables|/Script/Engine.Character|GetMesh _ownercharacter) (Utilities|Array|Get(acopy) (Variables|Default|GetAnimations) _sector)
    (:then
      (CallFunction|GetDirection))
    (:OnCompleted
      (Class|AbilityManagerComponent|TryDeactivateAvilitywithTag (Variables|/Script/RPG.CharacterBase|GetAbilityManagerComponent _ownercharacter) (Variables|Default|GetAbilityTag) :!label _label))
    (:OnInterrupted
      (goto _label))))

(event Custom|On%20Deactivate
  (params (AbilityGameplayTag :type Gameplay%20Tag%20Structure%20%28by%20ref%29) (AbilityPtr :type Character%20Ability%20Base%20Object%20Reference)))

(event Custom|On%20Interrupted
  (params (AbilityGameplayTag :type Gameplay%20Tag%20Structure%20%28by%20ref%29) (AbilityPtr :type Character%20Ability%20Base%20Object%20Reference)))

(event EventInitialize
  (params (InOwnerCharacter :type Character%20Base%20Object%20Reference))
  (|CallParentFunction InOwnerCharacter)
  (EventDispatchers|BindEventtoOnAbilityActivated (delegate Custom|On%20Activate))
  (EventDispatchers|BindEventtoOnAbilityDeactivated (delegate Custom|On%20Deactivate))
  (EventDispatchers|BindEventtoOnAbilityInterrputed (delegate Custom|On%20Interrupted)))

(fn GetDirection
  (bind _ownercharacter (Variables|Default|GetOwnerCharacter))
  (bind _returnvalue (Transformation|GetActorForwardVector _ownercharacter))
  (bind _returnvalue_2 (Pawn|GetMovementComponent _ownercharacter))
  (bind _returnvalue_3 (Pawn|Components|PawnMovement|GetLastInputVector _returnvalue_2))
  (bind _returnvalue_4 (Math|Vector|Normalize _returnvalue))
  (bind _returnvalue_5 (Math|Vector|Normalize _returnvalue_3))
  (bind _returnvalue_6 (Math|Vector|DotProduct _returnvalue_4 _returnvalue_5))
  (bind _returnvalue_7 (Class|KismetMathLibrary|DegAcos _returnvalue_6))
  (if (Utilities|Operators|EqualEqual _returnvalue_3 (Math|Vector|MakeVector 0.0 0.0 0.0) 1e-06)
    (return 0.0)
    (elif (> (Class|KismetMathLibrary|DegAsin (.z (Math|Vector|CrossProduct _returnvalue_4 _returnvalue_5))) 0.0)
      (return _returnvalue_7)
      (else
        (return (- 3.6e+02 _returnvalue_7))))))

(fn GetSector
  (params (angle :type Float%20%28double-precision%29))
  (return (Math|Float|Floor (Math|Float|SafeDivide (Math|Float|%(Float) (+ angle (Math|Float|SafeDivide 1.8e+02 (Math|Conversions|ToFloat(Integer) (Utilities|Array|Length (Variables|Default|GetAnimations))))) 3.6e+02) (Math|Float|SafeDivide 3.6e+02 (Math|Conversions|ToFloat(Integer) (Utilities|Array|Length (Variables|Default|GetAnimations))))))))

(fn RotateCharacter
  (bind _ownercharacter (Variables|Default|GetOwnerCharacter))
  (Transformation|SetActorRotation _ownercharacter (Pawn|GetControlRotation _ownercharacter :!class /Script/Engine.Pawn)))