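; Normal attack ability that plays a looping combo sequence of attack montages on the owning character.
; Each attack montage leads into a matching idle montage, during which the combo index advances and reactivation can chain the next hit.
; CanAttack blocks overlapping attacks and distinguishes a chained hit from other idle interruptions.
; Idle completion, unchained montage interruptions and ability interruption reset the combo, with montage endings also deactivating the ability by tag.
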(event Custom|On%20Activated
  (params (AvilityGameplayTag :type Gameplay%20Tag%20Structure%20%28by%20ref%29) (AbilityPtr :type Character%20Ability%20Base%20Object%20Reference))
  (bind _ownercharacter (Variables|Default|GetOwnerCharacter))
  (bind _mesh (Variables|/Script/Engine.Character|GetMesh _ownercharacter))
  (if (Variables|Default|GetCan%20Attack)
    (Variables|Default|SetCan%20Attack false)
    (Animation|Montage|PlayMontage _mesh (Utilities|Array|Get(acopy) (Variables|Default|GetAttack%20Montage) (Variables|Default|GetNext%20Attack%20Index))
      (:OnCompleted
        (Animation|Montage|PlayMontage _mesh (Utilities|Array|Get(acopy) (Variables|Default|GetIdle%20Montage) (Variables|Default|GetNext%20Attack%20Index))
          (:then
            (Variables|Default|SetNext%20Attack%20Index (Math|Integer|%(Integer) (+ (Variables|Default|GetNext%20Attack%20Index) 1) (Utilities|Array|Length (Variables|Default|GetAttack%20Montage))))
            (Variables|Default|SetCan%20Attack true))
          (:OnCompleted
            (Variables|Default|SetNext%20Attack%20Index 0 :!label _label)
            (Class|AbilityManagerComponent|TryDeactivateAvilitywithTag (Variables|/Script/RPG.CharacterBase|GetAbilityManagerComponent (Variables|Default|GetOwnerCharacter)) (Variables|Default|GetAbilityTag)))
          (:OnInterrupted
            (if (Variables|Default|GetCan%20Attack)
              (goto _label)))))
      (:OnInterrupted
        (Variables|Default|SetNext%20Attack%20Index 0)
        (Variables|Default|SetCan%20Attack true)
        (Class|AbilityManagerComponent|TryDeactivateAvilitywithTag (Variables|/Script/RPG.CharacterBase|GetAbilityManagerComponent (Variables|Default|GetOwnerCharacter)) (Variables|Default|GetAbilityTag))))))

(event Custom|On%20Deactivated
  (params (AvilityGameplayTag :type Gameplay%20Tag%20Structure%20%28by%20ref%29) (AbilityPtr :type Character%20Ability%20Base%20Object%20Reference)))

(event Custom|On%20Interrupted
  (params (AvilityGameplayTag :type Gameplay%20Tag%20Structure%20%28by%20ref%29) (AbilityPtr :type Character%20Ability%20Base%20Object%20Reference))
  (Variables|Default|SetCan%20Attack true)
  (Variables|Default|SetNext%20Attack%20Index 0))

(event EventInitialize
  (params (InOwnerCharacter :type Character%20Base%20Object%20Reference))
  (|CallParentFunction InOwnerCharacter)
  (EventDispatchers|BindEventtoOnAbilityActivated (delegate Custom|On%20Activated))
  (EventDispatchers|BindEventtoOnAbilityDeactivated (delegate Custom|On%20Deactivated))
  (EventDispatchers|BindEventtoOnAbilityInterrputed (delegate Custom|On%20Interrupted)))