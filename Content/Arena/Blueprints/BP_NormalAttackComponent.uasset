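; Actor component that runs the normal attack montage sequence for BP_ThirdPersonCharacter.
; Attack is gated by CanAttack and plays the attack montage at NextAttackIndex on the character mesh.
; On completion it starts the matching idle montage, advances the index with wraparound and immediately re-enables attacking as a combo window.
; The index resets when that idle montage completes or is interrupted, or when the attack is interrupted, which also re-enables attacking.
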(event Custom|Attack
  (if (Variables|Default|GetCan%20Attack)
    (bind _asbp_third_person_character (Utilities|Casting|CastToBP_ThirdPersonCharacter (Components|GetOwner)))
    (Variables|Default|SetCan%20Attack false)
    (Animation|Montage|PlayMontage (Variables|/Script/Engine.Character|GetMesh _asbp_third_person_character) (Utilities|Array|Get(acopy) (Variables|Default|GetAttack%20Montage) (Variables|Default|GetNext%20Attack%20Index))
      (:OnCompleted
        (Animation|Montage|PlayMontage (Variables|/Script/Engine.Character|GetMesh _asbp_third_person_character) (Utilities|Array|Get(acopy) (Variables|Default|GetIdle%20Montage) (Variables|Default|GetNext%20Attack%20Index))
          (:then
            (Variables|Default|SetNext%20Attack%20Index (Math|Integer|%(Integer) (+ (Variables|Default|GetNext%20Attack%20Index) 1) (Utilities|Array|Length (Variables|Default|GetAttack%20Montage))))
            (Variables|Default|SetCan%20Attack true))
          (:OnCompleted
            (Variables|Default|SetNext%20Attack%20Index 0 :!label _label))
          (:OnInterrupted
            (goto _label))))
      (:OnInterrupted
        (Variables|Default|SetNext%20Attack%20Index 0)
        (Variables|Default|SetCan%20Attack true)))))

(event EventBeginPlay)

(event EventTick
  (params (DeltaSeconds :type Float%20%28single-precision%29)))